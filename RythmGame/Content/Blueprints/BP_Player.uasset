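; BP_Player is a player Blueprint that resets its relative location on BeginPlay and spawns left, middle and right event key actors, apparently for a note-based rhythm game.
; Q, Z and D presses trigger the three spawn events, standing in for planned MIDI note input.
; The IA_Left, IA_Right and IA_Up handlers are empty, and an overlap debug print is unconnected.
; MoveAlongSpline only accumulates distance from DeltaTime and SplineSpeed.
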(event Custom|SpawnLeftEventKeys
  ;[1 1 1] Spawn event keys
  (Game|SpawnActorfromClass "/Game/Blueprints/BP_LeftEventKeys.BP_LeftEventKeys_C" (Math|Transform|MakeTransform "0, 0, 0" "0, 0, 0" "0.500000,0.500000,0.500000") "AlwaysSpawn" "OverrideRootScale" 0 0))

(event Custom|SpawnMiddleEventKeys
  ;[1 1 1] Spawn event keys
  (Game|SpawnActorfromClass "/Game/Blueprints/BP_MiddleEventKeys.BP_MiddleEventKeys_C" (Math|Transform|MakeTransform "0, 0, 0" "0, 0, 0" "0.500000,0.500000,0.500000") "AlwaysSpawn" "OverrideRootScale" 0 0))

(event Custom|SpawnRightEventKeys
  ;[1 1 1] Spawn event keys
  (Game|SpawnActorfromClass "/Game/Blueprints/BP_RightEventKeys.BP_RightEventKeys_C" (Math|Transform|MakeTransform "0.000000,0.000000,0.000000" "0, 0, 0" "0.550000,0.550000,0.550000") "AlwaysSpawn" "OverrideRootScale" 0 0))

(event Input|EnhancedActionEvents|EnhancedInputActionIA_Up
  (params (ActionValue :type Boolean) (ElapsedSeconds :type Float%20%28double-precision%29) (TriggeredSeconds :type Float%20%28double-precision%29) (InputAction :type Input%20Action%20Object%20Reference :default "/Game/Inputs/InputsAction/IA_Up.IA_Up"))
  ;[1 1 1] Get actor to make points
)

(event Input|EnhancedActionEvents|EnhancedInputActionIA_Left
  (params (ActionValue :type Boolean) (ElapsedSeconds :type Float%20%28double-precision%29) (TriggeredSeconds :type Float%20%28double-precision%29) (InputAction :type Input%20Action%20Object%20Reference :default "/Game/Inputs/InputsAction/IA_Left.IA_Left"))
  ;[1 1 1] Get actor to make points
)

(event Input|EnhancedActionEvents|EnhancedInputActionIA_Right
  (params (ActionValue :type Boolean) (ElapsedSeconds :type Float%20%28double-precision%29) (TriggeredSeconds :type Float%20%28double-precision%29) (InputAction :type Input%20Action%20Object%20Reference :default "/Game/Inputs/InputsAction/IA_Right.IA_Right"))
  ;[1 1 1] Get actor to make points
)

(event EventBeginPlay
  ;[1 1 1] Set player spawn to 0.0.0
  (Transformation|SetActorRelativeLocation "0, 0, 0"))

(event Input|KeyboardEvents|Z
  (params (Key :type Key%20Structure :default "None"))
  ;[1 1 1] Remplace input to midi note
  (:Pressed
    (CallFunction|SpawnMiddleEventKeys)))

(event Input|KeyboardEvents|Q
  (params (Key :type Key%20Structure :default "None"))
  ;[1 1 1] Remplace input to midi note
  (:Pressed
    (CallFunction|SpawnLeftEventKeys)))

(event Input|KeyboardEvents|D
  (params (Key :type Key%20Structure :default "None"))
  ;[1 1 1] Remplace input to midi note
  (:Pressed
    (CallFunction|SpawnRightEventKeys)))

(fn ConstructionScript)