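; BP_MiddleEventKeys is an actor that travels along the player's middle spline at a set speed.
; On BeginPlay it finds and stores the BP_Player instance as the spline source.
; Each Tick advances the travelled distance by SplineSpeed times delta time, then applies the world-space spline location and rotation to its root as a relative transform at half scale.
; The distance accumulates without wrapping or clamping.
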(event EventBeginPlay
  (bind _returnvalue (Actor|GetActorOfClass "/Game/Blueprints/BP_Player.BP_Player_C"))
  (Variables|Default|SetPlayerSpline _returnvalue))

(event EventTick
  (params (DeltaSeconds :type Float%20%28single-precision%29))
  (bind _distancealongspline (Variables|Default|GetDistanceAlongSpline))
  (bind _playerspline (Variables|Default|GetPlayerSpline))
  (bind _middlespline (Variables|/Game/Blueprints/BP_Player.BP_Player_C|GetMiddleSpline _playerspline))
  (bind _returnvalue (Spline|GetTransformatDistanceAlongSpline _middlespline _distancealongspline "World" false))
  (Utilities|MoveAlongSpline DeltaSeconds)
  (Transformation|SetRelativeTransform (Variables|Default|GetDefaultSceneRoot) (Math|Transform|MakeTransform (.location _returnvalue) (.rotation _returnvalue) "0.500000,0.500000,0.500000") false false))

(fn ConstructionScript)